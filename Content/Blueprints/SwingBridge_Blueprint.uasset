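; Swing bridge Blueprint that rotates the actor up and down around an arbitrary hinge axis.
; On Init, two hinge actors define the pivot and axis, and the starting offset and rotation are cached.
; SwingDown plays a timeline and SwingUp reverses it; while Enabled, each update rotates the cached offset and rotation by the timeline angle.
; An unreferenced helper computes the perpendicular vector from a point to a line.
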(event Custom|SwingDown_Event
  (bind _rotationaxis (Variables|Default|GetrotationAxis))
  (bind _angle (Timeline|SwingTimeline Play)
    (:Update
      (if (Variables|Default|Getenabled)
        (Transformation|SetActorLocationAndRotation (+ (Math|Vector|RotateVectorAroundAxis (Variables|Default|GetCenterOfRotationToActor) _angle _rotationaxis) (Variables|Default|GetcentreOfRotation)) (Math|Rotator|CombineRotators (Math|Vector|RotatorfromAxisandAngle _rotationaxis _angle) (Variables|Default|GetintialRotation)))))))

(event Custom|SwingUp_Event
  (bind _rotationaxis (Variables|Default|GetrotationAxis))
  (bind _angle (Timeline|SwingTimeline Reverse)
    (:Update
      (if (Variables|Default|Getenabled)
        (Transformation|SetActorLocationAndRotation (+ (Math|Vector|RotateVectorAroundAxis (Variables|Default|GetCenterOfRotationToActor) _angle _rotationaxis) (Variables|Default|GetcentreOfRotation)) (Math|Rotator|CombineRotators (Math|Vector|RotatorfromAxisandAngle _rotationaxis _angle) (Variables|Default|GetintialRotation)))))))

(event Custom|Init_Event
  (params (HingeAxisA :type Actor%20Object%20Reference) (AingeAxisB :type Actor%20Object%20Reference))
  (bind _returnvalue (Transformation|GetActorLocation HingeAxisA))
  (bind _output_get (Variables|Default|SetcentreOfRotation _returnvalue))
  (Variables|Default|SetrotationAxis (- _returnvalue (Transformation|GetActorLocation AingeAxisB)))
  (Variables|Default|SetCenterOfRotationToActor (- (Transformation|GetActorLocation) _output_get))
  (Variables|Default|SetintialRotation (Transformation|GetActorRotation))
  (EventDispatchers|BindEventtoSwingDown (delegate Custom|SwingDown_Event))
  (EventDispatchers|BindEventtoSwingUp (delegate Custom|SwingUp_Event)))

(event EventBeginPlay
  (|CallParentFunction)
  (EventDispatchers|BindEventtoInit (delegate Custom|Init_Event)))

(event Collision|EventActorBeginOverlap
  (params (OtherActor :type Actor%20Object%20Reference)))

(event EventTick
  (params (DeltaSeconds :type Float%20%28single-precision%29)))

(fn ConstructionScript)

(fn GetVectorfromPointtoLine
  (params (Line :type Vector) (Point :type Vector))
  (bind (_x _y _z) (Math|Vector|BreakVector Line))
  (bind (_x_2 _y_2 _z_2) (Math|Vector|BreakVector Point))
  (return (- (* Line (/ (+ (* _x _x_2) (* _y _y_2) (* _z _z_2)) (+ (Math|Float|Square _x) (Math|Float|Square _y) (Math|Float|Square _z)))) Point)))