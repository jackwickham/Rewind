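; Floor button actor that visibly sinks when pressed and rises back up when released.
; Press and release events fire the ButtonPressed and ButtonReleased dispatchers for any bound listeners.
; A timeline plays forward on press and reverses on release, offsetting the inner button component downward from its world position cached at BeginPlay.
; This graph contains no overlap detection, so OnButtonPress and OnButtonRelease must be triggered from elsewhere.
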(event EventBeginPlay
  (Variables|Default|SetbuttonStartLocation (Transformation|GetWorldLocation (Variables|Default|GetbuttonInnerComponent))))

(event Collision|EventActorBeginOverlap
  (params (OtherActor :type Actor%20Object%20Reference)))

(event EventTick
  (params (DeltaSeconds :type Float%20%28single-precision%29)))

(event EventOnButtonPress
  (Default|CallButtonPressed)
  (bind _multiplier (Timeline|buttonPressDown Play)
    (:Update
      (Transformation|SetWorldLocation (Variables|Default|GetbuttonInnerComponent) (+ (* "0, 0,-4.800000" _multiplier) (Variables|Default|GetbuttonStartLocation)) false))))

(event EventOnButtonRelease
  (Default|CallButtonReleased)
  (bind _multiplier (Timeline|buttonPressDown Reverse)
    (:Update
      (Transformation|SetWorldLocation (Variables|Default|GetbuttonInnerComponent) (+ (* "0, 0,-4.800000" _multiplier) (Variables|Default|GetbuttonStartLocation)) false))))

(fn ConstructionScript)