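; Movable bridge actor that slides along a path when triggered and supports the game's pause and rewind system.
; DoMove takes the offset between Start and End actors, and the MoveBridge timeline applies it from the bridge's current location.
; RewindGameMode pause and resume events stop and continue a partly done move.
; GetLocation adds timeline progress to the parent's history record; SetLocation restores it, resetting attached switches when rewound to zero.
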(event Custom|onResume_Event
  (params (time :type Float%20%28single-precision%29))
  (if (not (== (Components|Timeline|GetPlaybackPosition (Variables|Default|GetMove%20Bridge)) 0.0))
    (bind _multiplier (Timeline|Move%20Bridge Play)
      (:Update
        (Transformation|SetActorLocation (+ (* (Variables|Default|GetPath%20of%20Motion) _multiplier) (Variables|Default|GetBridge%20Start%20Location)) false)))))

(event Custom|DoMove_Event
  (params (Start :type Actor%20Object%20Reference) (End :type Actor%20Object%20Reference))
  (Variables|Default|SetPath%20of%20Motion (- (Transformation|GetActorLocation End) (Transformation|GetActorLocation Start)))
  (Variables|Default|SetBridge%20Start%20Location (Transformation|GetActorLocation))
  (bind _multiplier (Timeline|Move%20Bridge Play)
    (:Update
      (Transformation|SetActorLocation (+ (* (Variables|Default|GetPath%20of%20Motion) _multiplier) (Variables|Default|GetBridge%20Start%20Location)) false))))

(event Custom|onPause_Event
  (bind _multiplier (Timeline|Move%20Bridge Stop)
    (:Update
      (Transformation|SetActorLocation (+ (* (Variables|Default|GetPath%20of%20Motion) _multiplier) (Variables|Default|GetBridge%20Start%20Location)) false))))

(event EventBeginPlay
  (|CallParentFunction)
  (bind _asrewind_game_mode (Utilities|Casting|CastToRewindGameMode (Game|GetGameMode)))
  (EventDispatchers|BindEventtoOnPause _asrewind_game_mode (delegate Custom|onPause_Event))
  (EventDispatchers|BindEventtoDoMove (delegate Custom|DoMove_Event))
  (EventDispatchers|AssignOnResume _asrewind_game_mode (delegate Custom|onResume_Event)))

(event Collision|EventActorBeginOverlap
  (params (OtherActor :type Actor%20Object%20Reference)))

(event EventTick
  (params (DeltaSeconds :type Float%20%28single-precision%29)))

(event EventSetLocation
  (params (newState :type Location%20History%20Structure) (currentGameTime :type Integer))
  (bind _timelineprogress (Utilities|Struct|BreakLocationHistory newState))
  (if (== _timelineprogress 0.0)
    (if (!= (Components|Timeline|GetPlaybackPosition (Variables|Default|GetMove%20Bridge)) 0.0) ; To prevent a bug where setting it to 0 before it's been initialised caused the bridge to go to (0,0,0)
      (Default|CallResetAttachedSwitches)
      (bind _multiplier (Timeline|Move%20Bridge SetNewTime)
        (:Update
          (Transformation|SetActorLocation (+ (* (Variables|Default|GetPath%20of%20Motion) _multiplier) (Variables|Default|GetBridge%20Start%20Location)) false))))
    (else
      (Timeline|Move%20Bridge SetNewTime))))

(fn ConstructionScript)

(fn GetLocation
  (bind _returnvalue (|CallParentFunction))
  (return (Utilities|Struct|MakeLocationHistory (.timestamp (Utilities|Struct|BreakLocationHistory _returnvalue)) (.actor (Utilities|Struct|BreakLocationHistory _returnvalue)) (.lifespan (Utilities|Struct|BreakLocationHistory _returnvalue)) (.actorTransform (Utilities|Struct|BreakLocationHistory _returnvalue)) (.velocity (Utilities|Struct|BreakLocationHistory _returnvalue)) (Components|Timeline|GetPlaybackPosition (Variables|Default|GetMove%20Bridge)))))